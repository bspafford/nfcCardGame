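; Card Blueprint that drives the highlight of a five-slot card selection HUD through the 1–5 number keys.
; Each key calls removeSelection to reset every slot's border and font size, then gives its own slot the selected border and larger text.
; It only restyles CardSelectionWidget, which is not created here.
; The TempJoin widget code is unreachable, and BeginPlay and the testList RepNotify are empty.
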(event `self.tempBeginPlay`)

(event `removeSelection`
  (bind _cardselectionwidget (`self.cardSelectionWidget`))
  (`Image.SetBrush` (`cardSelectionWidget.slot1Image` _cardselectionwidget) (make `SlateBrush` "Image" "NoTile" "NoMirror" (struct :`X` 32.0 :`Y` 32.0) (struct) (struct :`SpecifiedColor` (struct :`R` 1.0 :`G` 1.0 :`B` 1.0 :`A` 1.0) :`ColorUseRule` "UseColor_Specified") (struct :`CornerRadii` (struct :`W` 1.0) :`Color` (struct :`SpecifiedColor` (struct) :`ColorUseRule` "UseColor_Specified") :`RoundingType` "HalfHeightRadius") "/Game/images/slotBorder.slotBorder"))
  (`TextBlock.SetFont` (`cardSelectionWidget.slot1Text` _cardselectionwidget) (make `SlateFontInfo` "/Engine/EngineFonts/Roboto.Roboto" null (struct :`OutlineColor` (struct :`A` 1.0)) "Bold" 52.0))
  (`Image.SetBrush` (`cardSelectionWidget.slot2Image` _cardselectionwidget) (make `SlateBrush` "Image" "NoTile" "NoMirror" (struct :`X` 32.0 :`Y` 32.0) (struct) (struct :`SpecifiedColor` (struct :`R` 1.0 :`G` 1.0 :`B` 1.0 :`A` 1.0) :`ColorUseRule` "UseColor_Specified") (struct :`CornerRadii` (struct :`W` 1.0) :`Color` (struct :`SpecifiedColor` (struct) :`ColorUseRule` "UseColor_Specified") :`RoundingType` "HalfHeightRadius") "/Game/images/slotBorder.slotBorder"))
  (`TextBlock.SetFont` (`cardSelectionWidget.slot2Text` _cardselectionwidget) (make `SlateFontInfo` "/Engine/EngineFonts/Roboto.Roboto" null (struct :`OutlineColor` (struct :`A` 1.0)) "Bold" 52.0))
  (`Image.SetBrush` (`cardSelectionWidget.slot3Image` _cardselectionwidget) (make `SlateBrush` "Image" "NoTile" "NoMirror" (struct :`X` 32.0 :`Y` 32.0) (struct) (struct :`SpecifiedColor` (struct :`R` 1.0 :`G` 1.0 :`B` 1.0 :`A` 1.0) :`ColorUseRule` "UseColor_Specified") (struct :`CornerRadii` (struct :`W` 1.0) :`Color` (struct :`SpecifiedColor` (struct) :`ColorUseRule` "UseColor_Specified") :`RoundingType` "HalfHeightRadius") "/Game/images/slotBorder.slotBorder"))
  (`TextBlock.SetFont` (`cardSelectionWidget.slot3Text` _cardselectionwidget) (make `SlateFontInfo` "/Engine/EngineFonts/Roboto.Roboto" null (struct :`OutlineColor` (struct :`A` 1.0)) "Bold" 52.0))
  (`Image.SetBrush` (`cardSelectionWidget.slot4Image` _cardselectionwidget) (make `SlateBrush` "Image" "NoTile" "NoMirror" (struct :`X` 32.0 :`Y` 32.0) (struct) (struct :`SpecifiedColor` (struct :`R` 1.0 :`G` 1.0 :`B` 1.0 :`A` 1.0) :`ColorUseRule` "UseColor_Specified") (struct :`CornerRadii` (struct :`W` 1.0) :`Color` (struct :`SpecifiedColor` (struct) :`ColorUseRule` "UseColor_Specified") :`RoundingType` "HalfHeightRadius") "/Game/images/slotBorder.slotBorder"))
  (`TextBlock.SetFont` (`cardSelectionWidget.slot4Text` _cardselectionwidget) (make `SlateFontInfo` "/Engine/EngineFonts/Roboto.Roboto" null (struct :`OutlineColor` (struct :`A` 1.0)) "Bold" 52.0))
  (`Image.SetBrush` (`cardSelectionWidget.slot5Image` _cardselectionwidget) (make `SlateBrush` "Image" "NoTile" "NoMirror" (struct :`X` 32.0 :`Y` 32.0) (struct) (struct :`SpecifiedColor` (struct :`R` 1.0 :`G` 1.0 :`B` 1.0 :`A` 1.0) :`ColorUseRule` "UseColor_Specified") (struct :`CornerRadii` (struct :`W` 1.0) :`Color` (struct :`SpecifiedColor` (struct) :`ColorUseRule` "UseColor_Specified") :`RoundingType` "HalfHeightRadius") "/Game/images/slotBorder.slotBorder"))
  (`TextBlock.SetFont` (`cardSelectionWidget.slot5Text` _cardselectionwidget) (make `SlateFontInfo` "/Engine/EngineFonts/Roboto.Roboto" null (struct :`OutlineColor` (struct :`A` 1.0)) "Bold" 52.0)))

(event `Key|One`
  (params (Key :type "Key Structure"))
  (bind _cardselectionwidget (`self.cardSelectionWidget`))
  (:`Pressed`
    (`self.removeSelection`)
    (`Image.SetBrush` (`cardSelectionWidget.slot1Image` _cardselectionwidget) (make `SlateBrush` "Image" "NoTile" "NoMirror" (struct :`X` 32.0 :`Y` 32.0) (struct) (struct :`SpecifiedColor` (struct :`R` 1.0 :`G` 1.0 :`B` 1.0 :`A` 1.0) :`ColorUseRule` "UseColor_Specified") (struct :`CornerRadii` (struct :`W` 1.0) :`Color` (struct :`SpecifiedColor` (struct) :`ColorUseRule` "UseColor_Specified") :`RoundingType` "HalfHeightRadius") "/Game/images/selectedSlotBorder.selectedSlotBorder"))
    (`TextBlock.SetFont` (`cardSelectionWidget.slot1Text` _cardselectionwidget) (make `SlateFontInfo` "/Engine/EngineFonts/Roboto.Roboto" null (struct :`OutlineColor` (struct :`A` 1.0)) "Bold" 60.0))))

(event `Key|Two`
  (params (Key :type "Key Structure"))
  (bind _cardselectionwidget (`self.cardSelectionWidget`))
  (:`Pressed`
    (`self.removeSelection`)
    (`Image.SetBrush` (`cardSelectionWidget.slot2Image` _cardselectionwidget) (make `SlateBrush` "Image" "NoTile" "NoMirror" (struct :`X` 32.0 :`Y` 32.0) (struct) (struct :`SpecifiedColor` (struct :`R` 1.0 :`G` 1.0 :`B` 1.0 :`A` 1.0) :`ColorUseRule` "UseColor_Specified") (struct :`CornerRadii` (struct :`W` 1.0) :`Color` (struct :`SpecifiedColor` (struct) :`ColorUseRule` "UseColor_Specified") :`RoundingType` "HalfHeightRadius") "/Game/images/selectedSlotBorder.selectedSlotBorder"))
    (`TextBlock.SetFont` (`cardSelectionWidget.slot2Text` _cardselectionwidget) (make `SlateFontInfo` "/Engine/EngineFonts/Roboto.Roboto" null (struct :`OutlineColor` (struct :`A` 1.0)) "Bold" 60.0))))

(event `Key|Three`
  (params (Key :type "Key Structure"))
  (bind _cardselectionwidget (`self.cardSelectionWidget`))
  (:`Pressed`
    (`self.removeSelection`)
    (`Image.SetBrush` (`cardSelectionWidget.slot3Image` _cardselectionwidget) (make `SlateBrush` "Image" "NoTile" "NoMirror" (struct :`X` 32.0 :`Y` 32.0) (struct) (struct :`SpecifiedColor` (struct :`R` 1.0 :`G` 1.0 :`B` 1.0 :`A` 1.0) :`ColorUseRule` "UseColor_Specified") (struct :`CornerRadii` (struct :`W` 1.0) :`Color` (struct :`SpecifiedColor` (struct) :`ColorUseRule` "UseColor_Specified") :`RoundingType` "HalfHeightRadius") "/Game/images/selectedSlotBorder.selectedSlotBorder"))
    (`TextBlock.SetFont` (`cardSelectionWidget.slot3Text` _cardselectionwidget) (make `SlateFontInfo` "/Engine/EngineFonts/Roboto.Roboto" null (struct :`OutlineColor` (struct :`A` 1.0)) "Bold" 60.0))))

(event `Key|Four`
  (params (Key :type "Key Structure"))
  (bind _cardselectionwidget (`self.cardSelectionWidget`))
  (:`Pressed`
    (`self.removeSelection`)
    (`Image.SetBrush` (`cardSelectionWidget.slot4Image` _cardselectionwidget) (make `SlateBrush` "Image" "NoTile" "NoMirror" (struct :`X` 32.0 :`Y` 32.0) (struct) (struct :`SpecifiedColor` (struct :`R` 1.0 :`G` 1.0 :`B` 1.0 :`A` 1.0) :`ColorUseRule` "UseColor_Specified") (struct :`CornerRadii` (struct :`W` 1.0) :`Color` (struct :`SpecifiedColor` (struct) :`ColorUseRule` "UseColor_Specified") :`RoundingType` "HalfHeightRadius") "/Game/images/selectedSlotBorder.selectedSlotBorder"))
    (`TextBlock.SetFont` (`cardSelectionWidget.slot4Text` _cardselectionwidget) (make `SlateFontInfo` "/Engine/EngineFonts/Roboto.Roboto" null (struct :`OutlineColor` (struct :`A` 1.0)) "Bold" 60.0))))

(event `Key|Five`
  (params (Key :type "Key Structure"))
  (bind _cardselectionwidget (`self.cardSelectionWidget`))
  (:`Pressed`
    (`self.removeSelection`)
    (`Image.SetBrush` (`cardSelectionWidget.slot5Image` _cardselectionwidget) (make `SlateBrush` "Image" "NoTile" "NoMirror" (struct :`X` 32.0 :`Y` 32.0) (struct) (struct :`SpecifiedColor` (struct :`R` 1.0 :`G` 1.0 :`B` 1.0 :`A` 1.0) :`ColorUseRule` "UseColor_Specified") (struct :`CornerRadii` (struct :`W` 1.0) :`Color` (struct :`SpecifiedColor` (struct) :`ColorUseRule` "UseColor_Specified") :`RoundingType` "HalfHeightRadius") "/Game/images/selectedSlotBorder.selectedSlotBorder"))
    (`TextBlock.SetFont` (`cardSelectionWidget.slot5Text` _cardselectionwidget) (make `SlateFontInfo` "/Engine/EngineFonts/Roboto.Roboto" null (struct :`OutlineColor` (struct :`A` 1.0)) "Bold" 60.0))))

(fn `OnRep_testList`)

(fn `UserConstructionScript`)