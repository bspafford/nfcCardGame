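; Game mode that assigns each player a spawn point from the CustomplayerStart actors placed in the level.
; On first use, InitializeSpawnPoints fills the SpawnPoints map, keyed by each start's player index.
; The ChoosePlayerStart override looks up the map with the current player count rather than the Player argument, with no fallback for a missing key.
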(fn `ChoosePlayerStart`
  (params (Player :type "Controller Object Reference"))
  (returns (ReturnValue :type "Actor Object Reference"))
  (`self.Initialize Spawn Points`)
  (bind _returnvalue (`self.GetNumPlayers`))
  (return (`BlueprintMapLibrary.Map_Find` (`self.spawnPoints`) _returnvalue)))

(fn `Initialize Spawn Points`
  (locals (NewLocalVar :type "PlayerStart Object Reference"))
  (if (== (`BlueprintMapLibrary.Map_Length` (`self.spawnPoints`)) 0)
    (bind _outactors (`GameplayStatics.GetAllActorsOfClass` "/Game/customplayerStart.customplayerStart_C"))
    (for _array_element _outactors
      (`BlueprintMapLibrary.Map_Add` (`self.spawnPoints`) (`/Game/customplayerStart.getPlayerIndex` _array_element) _array_element))))

(fn `UserConstructionScript`)